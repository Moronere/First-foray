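; Player controller for a PlayerVessel pawn that handles mouse camera control, cursor mode and the inventory toggle.
; On BeginPlay it caches the vessel and its HUD widget, then mouse axes accumulate scaled yaw and pitch into the control rotation.
; Cursor mode swaps between game-only input and Game-and-UI with vessel input disabled.
; ShowInventory opens or hides the inventory alongside cursor mode, while Escape only exits cursor mode.
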(event `self.ReceiveBeginPlay`
  ;[1 1 1] Initialization
  (bind _asplayer_vessel (cast `/Game/Blueprints/Characters/PlayerVessel` (`self.K2_GetPawn` self))
    (:`then`
      (bind _output_get (set `self.Controlled Player Vessel` _asplayer_vessel))
      (set `self.Player HUD Widget` (`/Game/Blueprints/Characters/PlayerVessel.HUD Widget` _output_get)))
    (:`CastFailed`
      (`KismetSystemLibrary.LogString` "WARNING! No Player Vessel assigned!"))))

(event `ActionMouseLeftRight`
  ;[0 0.2135 0.01313] Needs Work
)

(event `ActionMouseUpDown`
  ;[0 0.2135 0.01313] Needs Work
)

(event `EnhancedInput|/Game/Blueprints/Inputs/Escape`
  (params (ActionValue :type Boolean) (ElapsedSeconds :type "Float (double-precision)") (TriggeredSeconds :type "Float (double-precision)") (InputAction :type "InputAction Object Reference" :default "/Game/Blueprints/Inputs/Escape.Escape"))
  (:`Triggered`
    (if (`self.CursorMode`)
      (`self.Switch Cursor Mode`))))

(event `InputAxis|MouseLeftRight`
  (params (AxisValue :type "Float (single-precision)"))
  ;[1 1 1] Super Camera Control
  (bind _output_get (set `self.ControllerYaw` (+ (`self.ControllerYaw`) (* (`self.YawScale`) AxisValue))))
  (`self.SetControlRotation` (`KismetMathLibrary.MakeRotator` 0.0 (stale `InputAxis|MouseUpDown` _output_get) _output_get) :!label _label))

(event `InputAxis|MouseUpDown`
  (params (AxisValue :type "Float (single-precision)"))
  ;[1 1 1] Super Camera Control
  (bind _output_get (set `self.ControllerPitch` (+ (* AxisValue (`self.PitchScale`)) (`self.ControllerPitch`))))
  (goto _label))

(event `Switch Cursor Mode`
  (bind _controlled_player_vessel (`self.Controlled Player Vessel`))
  ;[0.5506 0.6559 1] UI
  (if (`self.CursorMode`)
    (`self.EnableInput` _controlled_player_vessel self)
    (`WidgetBlueprintLibrary.SetInputMode_GameOnly` self)
    (set `self.bShowMouseCursor` false)
    (set `self.CursorMode` false)
    (else
      (`self.DisableInput` _controlled_player_vessel self)
      (`WidgetBlueprintLibrary.SetInputMode_GameAndUIEx` self (`self.Player HUD Widget`) "LockOnCapture" false)
      (set `self.bShowMouseCursor` true)
      (set `self.CursorMode` true))))

(event `Close Windows`
  (bind _controlled_player_vessel (`self.Controlled Player Vessel`))
  ;[0.5506 0.6559 1] UI
  (if (> (+ (`/Game/Blueprints/Characters/PlayerVessel.InventoryOpen` (`self.Controlled Player Vessel`)) 0) 0)
    (`/Game/Blueprints/Components/InventorySystemComponent.Hide Inventory` (`/Game/Blueprints/Characters/PlayerVessel.InventoryComponent` _controlled_player_vessel) (`/Game/Blueprints/Characters/PlayerVessel.InventoryTilemap` _controlled_player_vessel) _controlled_player_vessel)
    (else
      (`KismetSystemLibrary.LogString` "No windows open."))))

(event `EnhancedInput|/Game/Blueprints/Inputs/ShowInventory`
  (params (ActionValue :type Boolean) (ElapsedSeconds :type "Float (double-precision)") (TriggeredSeconds :type "Float (double-precision)") (InputAction :type "InputAction Object Reference" :default "/Game/Blueprints/Inputs/ShowInventory.ShowInventory"))
  (bind _controlled_player_vessel (`self.Controlled Player Vessel`))
  ;[0.5506 0.6559 1] UI
  (:`Triggered`
    (if (`self.CursorMode`)
      (if (> (`/Game/Blueprints/Characters/PlayerVessel.InventoryOpen` _controlled_player_vessel) 0)
        (`self.Close Windows`)
        (`self.Switch Cursor Mode`)
        (else
          (`/Game/Blueprints/Characters/PlayerVessel.Open Inventory` _controlled_player_vessel :!label _label_2)))
      (else
        (`self.Switch Cursor Mode`)
        (goto _label_2)))))

(fn `UserConstructionScript`)
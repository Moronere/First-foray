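; Inventory component that lets the player scoop up nearby loot, with adding and removing items still unimplemented stubs.
; The Interact input runs LootScoop, a multi sphere trace centered on the player 0 pawn with a configurable radius.
; Each hit actor's InventoryItemComponent gets a LootMessage call without a validity check, and a trace with no blocking hit only logs that no loot was found.
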(event `EnhancedInput|/Game/Blueprints/Inputs/Interact`
  (params (ActionValue :type Boolean) (ElapsedSeconds :type "Float (double-precision)") (TriggeredSeconds :type "Float (double-precision)") (InputAction :type "InputAction Object Reference" :default "/Game/Blueprints/Inputs/Interact.Interact"))
  (:`Triggered`
    (`self.LootScoop`)))

(fn `AddItem`
  (params (`Item Name` :type Name) (Quantity :type Integer)))

(fn `LootScoop`
  (bind _returnvalue (`Actor.K2_GetActorLocation` (`GameplayStatics.GetPlayerPawn` 0)))
  (bind (_outhits _returnvalue_2) (`KismetSystemLibrary.SphereTraceMulti` _returnvalue _returnvalue (`self.ScoopRadius`) "TraceTypeQuery3"))
  (if _returnvalue_2
    (for _array_element _outhits
      (message `/Game/Blueprints/Interfaces/ILootInterface.Loot` (`Actor.GetComponentByClass` (`.HitActor` (`GameplayStatics.BreakHitResult` _array_element)) "/Game/Blueprints/Components/InventoryItemComponent.InventoryItemComponent_C")))
    (else
      (`KismetSystemLibrary.LogString` "No loot :("))))

(fn `RemoveItem`)
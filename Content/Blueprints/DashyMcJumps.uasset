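; DashyMcJumps is a player-controlled Blueprint that, as shown, handles only mouse-look camera control.
; Mouse axis inputs, multiplied by yaw and pitch scale variables, accumulate into stored ControllerYaw and ControllerPitch values that are applied through SetControlRotation with zero roll.
; Pitch input that would pass straight up or down is ignored rather than clamped to the limit.
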(event `InputAxis|MouseLeftRight`
  (params (AxisValue :type "Float (single-precision)"))
  ;[1 1 1] Super Camera Control
  (bind _output_get (set `self.ControllerYaw` (+ (`self.ControllerYaw`) (* (`self.InputYawScale`) AxisValue))))
  (`self.SetControlRotation` (`KismetMathLibrary.MakeRotator` 0.0 (stale `InputAxis|MouseUpDown` _output_get) _output_get) :!label _label))

(event `InputAxis|MouseUpDown`
  (params (AxisValue :type "Float (single-precision)"))
  (bind _returnvalue (+ (* AxisValue (`self.InputPitchScale`)) (`self.ControllerPitch`)))
  ;[1 1 1] Super Camera Control
  (if (and (<= _returnvalue 90.0) (>= _returnvalue -90.0))
    (bind _output_get (set `self.ControllerPitch` _returnvalue))
    (goto _label)))

(fn `UserConstructionScript`)